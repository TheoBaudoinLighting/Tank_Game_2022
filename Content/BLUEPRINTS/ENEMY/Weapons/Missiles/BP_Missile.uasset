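; BP_Missile is an enemy missile actor, apparently an early homing test, with most of its logic left disconnected.
; On a collision hit it only prints a debug message.
; Hit and Kill functions exist for explosion effects, sound and destruction, but no live path calls them.
; Unwired nodes sketch repeated lock-on, nearest "Homing"-tagged target search, ProjectileMovement homing and damage, while FindHomingTarget and the matching events are empty.
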(event `self.ReceiveBeginPlay`)

(event `ApplyDamage`
  ;[1 1 1] Test V01 Homing way
)

(event `self.ReceiveHit`
  (params (MyComp :type "PrimitiveComponent Object Reference") (Other :type "Actor Object Reference") (OtherComp :type "PrimitiveComponent Object Reference") (bSelfMoved :type Boolean) (HitLocation :type "Vector Structure") (HitNormal :type "Vector Structure") (NormalImpulse :type "Vector Structure") (Hit :type "HitResult Structure (by ref)"))
  ;[1 1 1] Test V01 Homing way
)

(event `self.Collision.OnComponentHit`
  (params (HitComponent :type "PrimitiveComponent Object Reference") (OtherActor :type "Actor Object Reference") (OtherComp :type "PrimitiveComponent Object Reference") (NormalImpulse :type "Vector Structure") (Hit :type "HitResult Structure (by ref)"))
  ;[1 1 1] Test V01 Homing way
  ;;[1 1 1] Missile logic
  (`KismetSystemLibrary.PrintString` "MISSILE HIT"))

(event `Lock On`
  ;[1 1 1] Test V01 Homing way
)

(fn `FindHomingTarget`
  (returns (HomingTarget :type "SceneComponent Object Reference")))

(fn `Hit`
  (bind _returnvalue (`SceneComponent.K2_GetComponentLocation` (`self.SM_Missile`)))
  (`GameplayStatics.SpawnEmitterAtLocation` "/Game/StarterContent/Particles/P_Explosion.P_Explosion" _returnvalue (struct) (5.0 5.0 5.0))
  (`GameplayStatics.PlaySoundAtLocation` "/Game/AUDIO/MINE/Mine_Cue.Mine_Cue" _returnvalue (struct) 1.0 1.0 0.0 null null null null)
  (`self.K2_DestroyActor`))

(fn `Kill`
  (`self.ApplyDamage`)
  (`self.K2_DestroyActor`))

(fn `UserConstructionScript`)