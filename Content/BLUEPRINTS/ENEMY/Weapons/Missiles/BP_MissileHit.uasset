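; Missile projectile actor that explodes on impact and self-destructs after three seconds.
; Hits spawn an explosion effect and sound, with radial damage added for Enemy, EnemyFast or Player tags, while other missiles are ignored.
; The damage origin is set from the hit's impact normal rather than its location.
; Tick moves MissileTarget to a forward trace's impact point as a homing test; FindHomingTarget is empty.
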(event `self.ReceiveBeginPlay`
  (`KismetSystemLibrary.Delay` 3.0)
  (`self.K2_DestroyActor`))

(event `self.ReceiveHit`
  (params (MyComp :type "PrimitiveComponent Object Reference") (Other :type "Actor Object Reference") (OtherComp :type "PrimitiveComponent Object Reference") (bSelfMoved :type Boolean) (HitLocation :type "Vector Structure") (HitNormal :type "Vector Structure") (NormalImpulse :type "Vector Structure") (Hit :type "HitResult Structure (by ref)"))
  ;[1 1 1] Test V01 Homing way
  (bind _output_get (set `self.Other` Other))
  (set `self.Hit Location` (`.ImpactNormal` (`GameplayStatics.BreakHitResult` Hit)))
  (`/Engine/EditorBlueprintResources/StandardMacros.IsValid` _output_get
    (:`Is Valid`
      (if (or (`self.ActorHasTag` _output_get "Enemy") (`self.ActorHasTag` _output_get "EnemyFast"))
        (`self.Hit`)
        (`self.Kill`)
        (elif (`self.ActorHasTag` _output_get "Player")
          (`self.Hit`)
          (`self.Kill`)
          (elif (not (`self.ActorHasTag` _output_get "Missile"))
            (`self.Hit`)))))))

(event `self.ReceiveTick`
  (params (DeltaSeconds :type "Float (single-precision)"))
  (bind _returnvalue (`self.K2_GetActorLocation`))
  (bind _outhit (`KismetSystemLibrary.LineTraceSingle` :`Start` _returnvalue :`End` (+ _returnvalue (* (`self.GetActorForwardVector`) 2000.0)) :`TraceChannel` "TraceTypeQuery1" :`DrawTime` 1.0))
  (`SceneComponent.K2_SetWorldLocation` (`self.MissileTarget`) (`.ImpactPoint` (`GameplayStatics.BreakHitResult` _outhit)) false false))

(fn `FindHomingTarget`)

(fn `Hit`
  (bind _returnvalue (`SceneComponent.K2_GetComponentLocation` (`self.SM_Missile`)))
  (`GameplayStatics.SpawnEmitterAtLocation` "/Game/StarterContent/Particles/P_Explosion.P_Explosion" _returnvalue (struct) (5.0 5.0 5.0))
  (`GameplayStatics.PlaySoundAtLocation` "/Game/AUDIO/MINE/Mine_Cue.Mine_Cue" _returnvalue (struct) 1.0 1.0 0.0 null null null null)
  (`self.K2_DestroyActor`))

(fn `Kill`
  (`GameplayStatics.ApplyRadialDamage` 200.0 (`self.Hit Location`) 150.0 null (`self.Ignore Actors`) self null)
  (`self.K2_DestroyActor`))

(fn `UserConstructionScript`)