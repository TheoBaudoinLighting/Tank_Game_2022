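; Enemy proximity mine that blinks at random intervals and explodes when a Player- or Bullet-tagged actor enters its explode area.
; A warning area speeds up the blink and adds a warning sound while the player is inside.
; The first blink also starts a one-time random fuse that detonates it regardless.
; Explosion spawns effects and destroys the actor; the separate damage event is never called here.
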(event `Flicker`
  ;[0 0.123 1] Mine base logic
  (`MeshComponent.SetScalarParameterValueOnMaterials` (`self.SM_Mine`) "Color" 100.0 :!label _label)
  (`KismetSystemLibrary.Delay` (`KismetMathLibrary.RandomFloatInRange` (`self.MinTimer`) (`self.MaxTimer`)))
  (`self.TurnOff`)
  (`/Engine/EditorBlueprintResources/StandardMacros.DoOnce` false
    (:`Completed`
      (`KismetSystemLibrary.Delay` (`KismetMathLibrary.RandomFloatInRange` 7.0 10.0))
      (`self.Explode`))))

(event `self.ReceiveBeginPlay`
  ;[0 0.123 1] Mine base logic
  (goto _label))

(event `TurnOff`
  ;[0 0.123 1] Mine base logic
  (if (`self.IsWarning?`)
    (`GameplayStatics.PlaySoundAtLocation` "/Game/AUDIO/MINE/MineRepeatWarning_Cue.MineRepeatWarning_Cue" (`SceneComponent.K2_GetComponentLocation` (`self.SM_Mine`)) (struct) 1.0 1.0 0.0 null null null null))
  (`MeshComponent.SetScalarParameterValueOnMaterials` (`self.SM_Mine`) "Color" 0.0)
  (`KismetSystemLibrary.Delay` (`KismetMathLibrary.RandomFloatInRange` (`self.MinTimer`) (`self.MaxTimer`)))
  (`self.Flicker`))

(event `self.WarningArea.OnComponentBeginOverlap`
  (params (OverlappedComponent :type "PrimitiveComponent Object Reference") (OtherActor :type "Actor Object Reference") (OtherComp :type "PrimitiveComponent Object Reference") (OtherBodyIndex :type Integer) (bFromSweep :type Boolean) (SweepResult :type "HitResult Structure (by ref)"))
  ;[1 0.9708 0.03164] Warning Area
  (bind _asbp_player (cast `/Game/BLUEPRINTS/PLAYER/BP_Player` OtherActor))
  (`/Engine/EditorBlueprintResources/StandardMacros.IsValid` _asbp_player
    (:`Is Valid`
      (set `self.MinTimer` 0.1)
      (set `self.MaxTimer` 0.2)
      (set `self.IsWarning?` true))))

(event `self.WarningArea.OnComponentEndOverlap`
  (params (OverlappedComponent :type "PrimitiveComponent Object Reference") (OtherActor :type "Actor Object Reference") (OtherComp :type "PrimitiveComponent Object Reference") (OtherBodyIndex :type Integer))
  ;[1 0.882 0] End Warning
  (bind _asbp_player (cast `/Game/BLUEPRINTS/PLAYER/BP_Player` OtherActor))
  (`/Engine/EditorBlueprintResources/StandardMacros.IsValid` _asbp_player
    (:`Is Valid`
      (set `self.MinTimer` 1.0)
      (set `self.MaxTimer` 2.0)
      (set `self.IsWarning?` false))))

(event `self.ExplodeArea.OnComponentBeginOverlap`
  (params (OverlappedComponent :type "PrimitiveComponent Object Reference") (OtherActor :type "Actor Object Reference") (OtherComp :type "PrimitiveComponent Object Reference") (OtherBodyIndex :type Integer) (bFromSweep :type Boolean) (SweepResult :type "HitResult Structure (by ref)"))
  ;[1 0 0] Explode Area
  (bind _output_get (set `self.Other Actor` OtherActor))
  (if (`self.ActorHasTag` _output_get "Player")
    (`self.Explode` :!label _label_2)
    (elif (`self.ActorHasTag` _output_get "Bullet")
      (goto _label_2))))

(event `Apply damage`
  ;[1 0 0] Apply damage
  (`GameplayStatics.ApplyDamage` (`self.Other Actor`) 200.0 null self))

(event `Explode`
  (bind _returnvalue (`SceneComponent.K2_GetComponentLocation` (`self.SM_Mine`)))
  ;[1 0 0] Exploding mine
  (`GameplayStatics.SpawnEmitterAtLocation` "/Game/StarterContent/Particles/P_Explosion.P_Explosion" _returnvalue (struct) (5.0 5.0 5.0))
  (`GameplayStatics.PlaySoundAtLocation` "/Game/AUDIO/MINE/Mine_Cue.Mine_Cue" _returnvalue (struct) 1.0 1.0 0.0 null null null null)
  (`self.K2_DestroyActor`))

(fn `UserConstructionScript`)