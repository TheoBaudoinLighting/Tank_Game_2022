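; BP_Enemy_01 is a basic enemy Blueprint that takes damage and is destroyed when its health runs out.
; On BeginPlay it calls the parent logic and caches the player character as a BP_Player reference.
; AnyDamage subtracts damage from Health and destroys the actor only when Health equals exactly zero.
; An ACShootSystem Shoot call exists in the graph but is not connected to any event.
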(event `self.ReceiveBeginPlay`
  ;[1 1 1] Set up base Enemy
  (`parent.ReceiveBeginPlay`)
  (bind _asbp_player (cast `/Game/BLUEPRINTS/PLAYER/BP_Player` (`GameplayStatics.GetPlayerCharacter` 0)))
  (set `self.Char REF` _asbp_player))

(event `self.ReceiveAnyDamage`
  (params (Damage :type "Float (single-precision)") (DamageType :type "DamageType Object Reference") (InstigatedBy :type "Controller Object Reference") (DamageCauser :type "Actor Object Reference"))
  ;[1 0 0] Set up health and damage
  (bind _output_get (set `self.Health` (- (`self.Health`) Damage)))
  (if (== _output_get 0.0)
    (`self.K2_DestroyActor`)))

(fn `UserConstructionScript`)