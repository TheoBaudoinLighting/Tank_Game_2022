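; BP_Enemy_03 is an enemy Blueprint that can lay mines and is destroyed by any damage it takes.
; On BeginPlay it runs its parent setup, then caches the player character as a BP_Player reference.
; Its PlacingBomb event spawns a BP_Mine at the mesh's world location, ignoring collision, though nothing in this graph calls that event.
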(event `self.ReceiveBeginPlay`
  ;[1 1 1] Set up base Enemy
  (`parent.ReceiveBeginPlay`)
  (bind _asbp_player (cast `/Game/BLUEPRINTS/PLAYER/BP_Player` (`GameplayStatics.GetPlayerCharacter` 0)))
  (set `self.Char REF` _asbp_player))

(event `self.ReceiveAnyDamage`
  (params (Damage :type "Float (single-precision)") (DamageType :type "DamageType Object Reference") (InstigatedBy :type "Controller Object Reference") (DamageCauser :type "Actor Object Reference"))
  ;[1 0 0] Set up health and damage
  (`self.K2_DestroyActor`))

(event `PlacingBomb`
  ;[1 0.9839 0] Placing bomb
  (`|SpawnActorFromClass` "/Game/BLUEPRINTS/ENEMY/Weapons/BP_Mine.BP_Mine_C" (`KismetMathLibrary.MakeTransform` (`SceneComponent.K2_GetComponentLocation` (`self.Mesh`))) "AlwaysSpawn" "OverrideRootScale" null null))

(fn `UserConstructionScript`)