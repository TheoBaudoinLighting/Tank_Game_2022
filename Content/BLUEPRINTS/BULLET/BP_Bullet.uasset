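; Bullet actor that damages enemies and players on hit and can bounce off other surfaces.
; Hit checks the actor tag, then ApplyDomage deals a fixed amount of damage and destroys the bullet, with a debug print.
; Other hits on non-simulating components increment HitNumber through a short retriggerable delay that merges rapid contacts, destroying the bullet once the count has reached three.
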(event `self.ReceiveHit`
  (params (MyComp :type "PrimitiveComponent Object Reference") (Other :type "Actor Object Reference") (OtherComp :type "PrimitiveComponent Object Reference") (bSelfMoved :type Boolean) (HitLocation :type "Vector Structure") (HitNormal :type "Vector Structure") (NormalImpulse :type "Vector Structure") (Hit :type "HitResult Structure (by ref)"))
  ;[0.1667 0.1667 0.1667] Bullet Logic
  (set `self.Other` Other)
  (set `self.Other Comp` OtherComp)
  ;;[1 0 0.8687] Check if collide with the enemy
  (if (`self.ActorHasTag` (`self.Other`) (`self.TagEnemy`))
    (`self.ApplyDomage`)
    (`KismetSystemLibrary.PrintString` "Hit Enemy")
    (else
      ;;[0 0.07764 1] Check if collide with player
      (if (`self.ActorHasTag` (`self.Other`) (`self.TagPlayer`))
        (`self.ApplyDomage`)
        (`KismetSystemLibrary.PrintString` "Hit Player")
        (else
          ;;[0 1 0.1344] Calculate number of bounces
          (if (`SceneComponent.IsSimulatingPhysics` (`self.Other Comp`) "None")
            _
            (elif (>= (`self.HitNumber`) 3)
              (`self.K2_DestroyActor`)
              (else
                (`KismetSystemLibrary.RetriggerableDelay` 0.1)
                (bind _result (`/Engine/EditorBlueprintResources/StandardMacros.IncrementInt` (`self.HitNumber`)))))))))))

(event `ApplyDomage`
  ;[0.1667 0.1667 0.1667] Bullet Logic
  ;;[1 0 0.03818] Apply Dammage
  (`GameplayStatics.ApplyDamage` (`self.Other`) 100.0 null self)
  (`self.K2_DestroyActor`))

(fn `UserConstructionScript`)