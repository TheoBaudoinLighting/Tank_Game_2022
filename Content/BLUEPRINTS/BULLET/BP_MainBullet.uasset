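; Main bullet actor that damages tagged players or enemies, bursts against other bullets and ricochets off other surfaces.
; On hit, actor tags route to shared Hit and Kill events for explosion FX, sounds, fixed damage and destruction.
; Other impacts increment a bounce counter behind a short retriggerable delay, exploding the bullet once the limit is reached.
; A BeginPlay timer also destroys it after a fixed lifetime.
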(event `self.ReceiveBeginPlay`
  ;[0.9326 0.6013 1] Destroy actor after some time
  (`KismetSystemLibrary.Delay` 10.0)
  (`self.K2_DestroyActor`))

(event `ApplyDamage`
  ;[1 0 0.03818] Apply Dammage
  (`GameplayStatics.ApplyDamage` (`self.Other`) 200.0 null self)
  (`self.K2_DestroyActor`))

(event `self.ReceiveHit`
  (params (MyComp :type "PrimitiveComponent Object Reference") (Other :type "Actor Object Reference") (OtherComp :type "PrimitiveComponent Object Reference") (bSelfMoved :type Boolean) (HitLocation :type "Vector Structure") (HitNormal :type "Vector Structure") (NormalImpulse :type "Vector Structure") (Hit :type "HitResult Structure (by ref)"))
  (bind _other (`self.Other`))
  ;[0.1667 0.1667 0.1667] Bullet Logic
  (bind _output_get (set `self.Other` Other))
  (set `self.Other Comp` OtherComp)
  (set `self.Hit Location` HitLocation)
  (`/Engine/EditorBlueprintResources/StandardMacros.IsValid` _output_get
    (:`Is Valid`
      ;;[1 0 0.8687] Check if collide with the enemy
      (if (`self.ActorHasTag` _output_get "Enemy")
        (`self.Hit`)
        (`self.Kill`)
        (else
          ;;[1 0.9258 0] Check if collide with the player
          (if (`self.ActorHasTag` (`self.Other`) "Player")
            (`self.Hit`)
            (`self.Kill`)
            (else
              ;;[1 0 0] Bullet over bullet logic
              (if (`self.ActorHasTag` _other "BulletPlayer")
                (`self.Hit`)
                (elif (`self.ActorHasTag` _other "BulletEnemy")
                  (`self.Hit`)
                  (else
                    ;;[0 1 0.1344] Calculate number of bounces
                    (if (>= (`self.HitNumber`) 3)
                      (`self.Hit`)
                      (else
                        (`KismetSystemLibrary.RetriggerableDelay` 0.1)
                        (bind _result (`/Engine/EditorBlueprintResources/StandardMacros.IncrementInt` (`self.HitNumber`))
                          (:`  `
                            (`GameplayStatics.PlaySoundAtLocation` "/Game/AUDIO/BULLET/Bounce_Cue.Bounce_Cue" (`self.Hit Location`) (struct) 1.0 1.0 0.0 null null null null)))))))))))))
    (:`Is Not Valid`
      (set `self.Other` _output_get)
      (set `self.Hit Location` HitLocation))))

(event `Kill`
  ;[1 1 1] Kill pawn
  (`self.ApplyDamage`)
  (`GameplayStatics.PlaySound2D` "/Game/AUDIO/BULLET/Hit_Cue.Hit_Cue" 1.0 1.0 0.0 null null)
  (`self.K2_DestroyActor`))

(event `Hit`
  ;[1 1 1] Hit
  (`GameplayStatics.PlaySoundAtLocation` "/Game/AUDIO/BULLET/Hit_Cue.Hit_Cue" (`self.Hit Location`) (struct) 1.0 1.0 0.0 null null null null)
  (`NiagaraFunctionLibrary.SpawnSystemAtLocation` "/Game/FX/BULLET/FX_BulletExplode.FX_BulletExplode" (`self.Hit Location`))
  (`self.K2_DestroyActor`))

(fn `UserConstructionScript`)