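; Animation notify state "BulletAttack" that deals bullet damage to pawns during its animation window.
; Each tick, it box-traces in place at the mesh's Bullet_Joint socket, oriented to that socket, for Pawn objects.
; The hit actor receives base damage and joins an ignore list, so it is damaged once per window.
; The list clears when the notify ends.
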(fn `GetNotifyName`
  (returns (ReturnValue :type String))
  (return "BulletAttack"))

(fn `Received_NotifyEnd`
  (params (MeshComp :type "SkeletalMeshComponent Object Reference") (Animation :type "AnimSequenceBase Object Reference"))
  (returns (ReturnValue :type Boolean))
  (`KismetArrayLibrary.Array_Clear` (`self.Actors to Ignore`))
  (return false))

(fn `Received_NotifyTick`
  (params (MeshComp :type "SkeletalMeshComponent Object Reference") (Animation :type "AnimSequenceBase Object Reference") (FrameDeltaTime :type "Float (double-precision)"))
  (returns (ReturnValue :type Boolean))
  (bind (_returnvalue_location _returnvalue_rotation) (`KismetMathLibrary.BreakTransform` (`SceneComponent.GetSocketTransform` MeshComp "Bullet_Joint" "RTS_World")))
  (bind _outhit (`KismetSystemLibrary.BoxTraceSingleForObjects` MeshComp _returnvalue_location _returnvalue_location (`self.Half Size`) _returnvalue_rotation (`|MakeArray` "ObjectTypeQuery3" :!type "EObjectTypeQuery Enum") false (`self.Actors to Ignore`) (`self.Draw Debug Type`)))
  (bind (_bblockinghit _binitialoverlap _time _distance _location _impactpoint _normal _impactnormal _physmat _hitactor) (`GameplayStatics.BreakHitResult` _outhit))
  (`KismetArrayLibrary.Array_AddUnique` (`self.Actors to Ignore`) _hitactor)
  (bind _returnvalue (`GameplayStatics.ApplyDamage` _hitactor (`self.Base Damage`)))
  (if (== _returnvalue 100.0)
    _
    (else
      _))
  (return false))