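; Dynamic light Blueprint with a sphere mesh, built to blink on and off, though nothing in its own graph starts the blink.
; BeginPlay gives the sphere a dynamic material instance.
; TurnOn and TurnOff would toggle a BP_DirectionalLight and sphere visibility, re-triggering each other on two-second timers, but their casts have no object connected.
; Disconnected leftovers include random color changes and delayed toggles.
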(event `self.ReceiveBeginPlay`
  (bind _returnvalue (`PrimitiveComponent.CreateDynamicMaterialInstance` (`self.Sphere`) 0 null "None"))
  (bind _output_get (set `self.DynamicMat` _returnvalue))
  (`PrimitiveComponent.SetMaterial` (`self.Sphere`) 0 _output_get))

(event `TurnOn`
  (bind _asbp_directional_light (cast `/Game/BLUEPRINTS/LIGHT/BP_DirectionalLight` null))
  (`/Game/BLUEPRINTS/LIGHT/BP_DirectionalLight.TurnOn` _asbp_directional_light)
  (`SceneComponent.SetVisibility` (`self.Sphere`) true false)
  (`KismetSystemLibrary.K2_SetTimer` null "TurnOff" 2.0))

(event `TurnOff`
  (bind _asbp_directional_light (cast `/Game/BLUEPRINTS/LIGHT/BP_DirectionalLight` null))
  (`/Game/BLUEPRINTS/LIGHT/BP_DirectionalLight.TurnOff` _asbp_directional_light)
  (`SceneComponent.SetVisibility` (`self.Sphere`) false false)
  (`KismetSystemLibrary.K2_SetTimer` null "TurnOn" 2.0))

(event `self.ReceiveTick`
  (params (DeltaSeconds :type "Float (single-precision)")))

(fn `UserConstructionScript`)