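; BP_Gamemode is the game mode that sets up local multiplayer players and a shared camera when play begins.
; SpawnPlayers creates a local player for each index between MinPlayers and MaxPlayers, then spawns a BP_Player pawn at a fixed location for each controller to possess.
; It then takes the first BP_Camera found in the level and sets it as player 0's view target.
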(event `self.ReceiveBeginPlay`
  ;[1 1 1] Setup Game
  (`|ExecutionSequence`
    (:`then_0`
      (`self.SpawnPlayers`)
      (`self.Find Camera Actor`))
    (:`then_1`
      (`PlayerController.SetViewTargetWithBlend` (`GameplayStatics.GetPlayerController` 0) (`self.MainCamera`) 0.0 "VTBlend_Linear" 0.0 false))))

(event `Find Camera Actor`
  ;[1 1 1] Find Camera For each actor
  (bind _outactors (`GameplayStatics.GetAllActorsOfClass` "/Game/BLUEPRINTS/BASE_BP/BP_Camera.BP_Camera_C"))
  (set `self.MainCamera` (`|GetArrayItem` _outactors)))

(fn `SpawnPlayers`
  (bind _min_players (`self.Min Players`))
  (bind _max_players (`self.Max Players`))
  ;[0 1 0.2089] Spawning Players
  (for _index (range _min_players (+ _max_players 1))
    ;;[0 0.1587 1] Create player by Index
    (`GameplayStatics.CreatePlayer` _index))
  (for _index_2 (range _min_players (+ _max_players 1))
    (bind _returnvalue (`|SpawnActorFromClass` "/Game/BLUEPRINTS/PLAYER/BP_Player.BP_Player_C" (`KismetMathLibrary.MakeTransform` (0.0 0.0 200.0)) "Undefined" "OverrideRootScale" null null))
    (`Controller.Possess` (`GameplayStatics.GetPlayerController` _index_2) _returnvalue)))

(fn `UserConstructionScript`)