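; Actor component that gives the player's tank its cannon shot.
; Its Shoot function casts the player pawn to BP_Player, plays the tank firing montage and spawns a BP_Bullet at the mesh's Canon_Joint socket, always spawning regardless of collision.
; A cannon sound plays at the socket location.
; The shot always targets player 0's pawn rather than the component's owner, and the event graph is unused.
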(fn `Shoot`
  (bind _worldtransform_location (`KismetMathLibrary.BreakTransform` (`self.WorldTransform`)))
  (bind _asbp_player (cast `/Game/BLUEPRINTS/PLAYER/BP_Player` (`GameplayStatics.GetPlayerPawn` 0)))
  (bind _output_get (set `self.Character` _asbp_player))
  (`Character.PlayAnimMontage` _output_get "/Game/ANIMATION/TANK/Tank_Shoot_Montage.Tank_Shoot_Montage" 1.0 "None")
  (bind _returnvalue (`SceneComponent.GetSocketTransform` (`Character.Mesh` _asbp_player) "Canon_Joint" "RTS_World"))
  (set `self.WorldTransform` _returnvalue)
  (`|SpawnActorFromClass` "/Game/BLUEPRINTS/BULLET/BP_Bullet.BP_Bullet_C" _returnvalue "AlwaysSpawn" "OverrideRootScale" null null)
  (`GameplayStatics.PlaySoundAtLocation` "/Game/AUDIO/TANK/Canon_shot_cue.Canon_shot_cue" _worldtransform_location (struct) 0.2 1.0 0.0 null null null null)
  (return))