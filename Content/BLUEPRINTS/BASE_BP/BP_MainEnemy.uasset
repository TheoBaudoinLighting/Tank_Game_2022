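; Base enemy tank Character that aims its turret at the player, fires when AI calls it, and explodes on any damage.
; Tick updates turret yaw toward a look-at point, which follows the player while visible, and runs line traces to set CanShoot.
; AI_ShootPlayer plays a montage and fires from BulletDirection through the ACShootSystem component.
; Damage has no health check: the first hit spawns effects and destroys the actor.
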(event `self.ReceiveBeginPlay`
  ;[0.4549 0.5912 1] Set Speed
  (set `CharacterMovementComponent.MaxWalkSpeed` (`self.MaxWalkSpeed`) (`self.CharacterMovement`)))

(event `self.ReceiveTick`
  (params (DeltaSeconds :type "Float (single-precision)"))
  (bind _returnvalue (`GameplayStatics.GetPlayerCharacter` 0))
  (bind _returnvalue_2 (`SceneComponent.K2_GetComponentLocation` (`self.BulletDirection`)))
  (bind _returnvalue_3 (`SceneComponent.K2_GetComponentLocation` (`Character.Mesh` _returnvalue)))
  ;[0 0.03342 1] Target Logic Any Tank
  (`self.TurretAiming`)
  (`/Engine/EditorBlueprintResources/StandardMacros.IsValid` _returnvalue
    (:`Is Valid`
      (`|ExecutionSequence`
        (:`then_0`
          (bind (_outhit _returnvalue_4) (`KismetSystemLibrary.LineTraceSingleForObjects` :`Start` _returnvalue_2 :`End` _returnvalue_3 :`ObjectTypes` (`self.Object Types`) :`DrawTime` 1.0))
          (if (and _returnvalue_4 (not (stale _returnvalue_5)))
            (if (`self.ActorHasTag` (`GameplayStatics.GetPlayerCharacter` 0) "Player")
              (set `self.CanShoot?` true)
              (else
                (set `self.CanShoot?` false)))
            (if (`self.IsPlayerVisilble?`)
              (set `self.TurretLookAt` (`SceneComponent.K2_GetComponentLocation` (`Character.Mesh` (`GameplayStatics.GetPlayerCharacter` 0))))
              (else
                (set `self.TurretLookAt` (`SceneComponent.K2_GetComponentLocation` (`self.Mesh`)))))))
        (:`then_1`
          (bind (_outhit_2 _returnvalue_5) (`KismetSystemLibrary.LineTraceSingle` :`Start` _returnvalue_3 :`End` _returnvalue_2 :`TraceChannel` "TraceTypeQuery1" :`DrawTime` 2.0)))))))

(event `self.ReceiveAnyDamage`
  (params (Damage :type "Float (single-precision)") (DamageType :type "DamageType Object Reference") (InstigatedBy :type "Controller Object Reference") (DamageCauser :type "Actor Object Reference"))
  (bind _returnvalue (`SceneComponent.K2_GetComponentLocation` (`self.Mesh`)))
  ;[1 0.09604 0] Die logic
  (`GameplayStatics.SpawnEmitterAtLocation` "/Game/StarterContent/Particles/P_Explosion.P_Explosion" _returnvalue (struct) (5.0 5.0 5.0))
  (`NiagaraFunctionLibrary.SpawnSystemAtLocation` "/Game/FX/TANK/NS_Explosion.NS_Explosion" _returnvalue (struct) (2.0 2.0 2.0))
  (`GameplayStatics.PlaySoundAtLocation` "/Game/AUDIO/MINE/Mine_Cue.Mine_Cue" (0.0 0.0 0.0) (struct) 1.0 1.0 0.0 null null null null)
  (`self.K2_DestroyActor`))

(event `AI_ShootPlayer`
  (params (Owner :type "Pawn Object Reference"))
  (bind _bulletdirection (`self.BulletDirection`))
  ;[1 1 1] Shoot AI logic
  (`self.PlayAnimMontage` "/Game/ANIMATION/TANK/Tank_Shoot_Montage.Tank_Shoot_Montage")
  (`/Game/BLUEPRINTS/BASE_BP/AC_Tank/AC_ShootSystem.Shoot` (`self.AC_ShootSystem`) (`KismetMathLibrary.MakeTransform` (`SceneComponent.K2_GetComponentLocation` _bulletdirection) (`KismetMathLibrary.MakeRotFromZ` (`SceneComponent.GetForwardVector` _bulletdirection))) Owner (`self.AIShotColorDebug`) (`self.CapsuleComponent`)))

(event `SetTurretLookAt`
  (params (TurretLookAt :type "Vector Structure"))
  ;[1 1 1] set turret look at
  (set `self.TurretLookAt` TurretLookAt))

(fn `TurretAiming`
  (bind (_returnvalue_roll _returnvalue_pitch _returnvalue_yaw) (`KismetMathLibrary.BreakRotator` (`KismetMathLibrary.FindLookAtRotation` (`self.TurretLookAt`) (`SceneComponent.GetSocketLocation` (`self.Mesh`) "Turret_Joint"))))
  ;[1 1 1] Aiming logic
  (set `self.ZOffset` _returnvalue_yaw))

(fn `UserConstructionScript`)