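; Base tank Character Blueprint that sets its walk speed and tracks the player for turret aiming.
; BeginPlay copies MaxWalkSpeed into CharacterMovement.
; Every Tick, TurretAiming casts player pawn 0 to BP_Player and stores in ZOffset the look-at yaw from the player's mesh to the Turret_Joint socket.
; The Blueprint only computes this yaw and does not rotate the turret itself.
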(event `self.ReceiveBeginPlay`
  ;[0.4549 0.5912 1] Set Speed
  (set `CharacterMovementComponent.MaxWalkSpeed` (`self.MaxWalkSpeed`) (`self.CharacterMovement`)))

(event `self.ReceiveTick`
  (params (DeltaSeconds :type "Float (single-precision)"))
  ;[0 0.03342 1] Target Logic Any Tank
  (`self.TurretAiming`))

(fn `TurretAiming`
  (bind _asbp_player (cast `/Game/BLUEPRINTS/PLAYER/BP_Player` (`GameplayStatics.GetPlayerPawn` 0)))
  (bind (_returnvalue_roll _returnvalue_pitch _returnvalue_yaw) (`KismetMathLibrary.BreakRotator` (`KismetMathLibrary.FindLookAtRotation` (`SceneComponent.K2_GetComponentLocation` (`Character.Mesh` _asbp_player)) (`SceneComponent.GetSocketLocation` (`self.Mesh`) "Turret_Joint"))))
  (set `self.ZOffset` _returnvalue_yaw))

(fn `UserConstructionScript`)