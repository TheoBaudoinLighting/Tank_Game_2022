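; Camera actor with a spring arm that records reference positions for itself and the first player character.
; On BeginPlay it caches that character, the spring arm's world X and Y, and a start vector holding only the actor's height.
; The SetCenterPoint event stores the character's current location as the center position.
; These graphs only store values; none of them moves the camera or calls SetCenterPoint.
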(event `self.ReceiveBeginPlay`
  ;[0 0.4807 1] Set Camera Position
  (`|ExecutionSequence`
    (:`then_0`
      (set `self.Character_01` (`GameplayStatics.GetPlayerCharacter` 0)))
    (:`then_1`
      (set `self.CameraYPos` (.y (`SceneComponent.K2_GetComponentLocation` (`self.SpringArm`))))
      (set `self.CameraXPos` (.x (`SceneComponent.K2_GetComponentLocation` (`self.SpringArm`))))
      (set `self.CameraStartPosition` (`KismetMathLibrary.MakeVector` 0.0 0.0 (.z (`self.K2_GetActorLocation`)))))))

(event `SetCenterPoint`
  ;[1 0.3687 0] Set Center Point Player
  (set `self.CenterPosition` (`self.K2_GetActorLocation` (`self.Character_01`))))

(fn `UserConstructionScript`)