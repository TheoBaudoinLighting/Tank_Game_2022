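; AC_ShootSystem is a tank component that fires cannon shells for player and enemy tanks.
; Shoot reads the owner's Player, Enemy or EnemyFast tag to select the matching bullet Blueprint class, and does nothing for untagged owners.
; It spawns the bullet at the supplied cannon transform regardless of collision and plays a quiet cannon shot sound.
; The Color input is unused, and the event graph is empty.
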(fn `Shoot`
  (params (`Canon Transform` :type "Transform Structure") (Owner :type "Pawn Object Reference") (Color :type "LinearColor Structure"))
  (bind _worldtransform_location (`KismetMathLibrary.BreakTransform` (`self.WorldTransform`)))
  (if (`Actor.ActorHasTag` Owner "Player")
    (set `self.Index` 0)
    (`|SpawnActorFromClass` (select `int` (`self.Index`) :`0` "/Game/BLUEPRINTS/BULLET/BP_BulletPlayer.BP_BulletPlayer_C" :`1` "/Game/BLUEPRINTS/BULLET/BP_BulletEnemy.BP_BulletEnemy_C" :`2` "/Game/BLUEPRINTS/BULLET/BP_BulletEnemyFast.BP_BulletEnemyFast_C" :!type "Actor Class Reference") `Canon Transform` "AlwaysSpawn" "OverrideRootScale" null null :!label _label)
    (`GameplayStatics.PlaySoundAtLocation` "/Game/AUDIO/TANK/Canon_shot_cue.Canon_shot_cue" _worldtransform_location (struct) 0.2 1.0 0.0 null null null null)
    (return)
    (elif (`Actor.ActorHasTag` Owner "Enemy")
      (set `self.Index` 1)
      (goto _label)
      (elif (`Actor.ActorHasTag` Owner "EnemyFast")
        (set `self.Index` 2)
        (goto _label)))))