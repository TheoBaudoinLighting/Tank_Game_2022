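; Tank motor component that turns forward and right axis input into player pawn movement and tracks scrolling UV offsets for the treads.
; Both handlers add movement input along the control rotation's yaw-only forward or right vector, scaled by speed, and record position and turn offsets.
; UpdateTreadUVs accumulates these per tread, weighting turn by each side's direction, then converts them to UV offsets using tread length and tiling.
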(event `Forward Handler`
  (params (Axis :type "Float (double-precision)"))
  (bind _returnvalue (`GameplayStatics.GetPlayerPawn` 0))
  (bind _returnvalue_2 (* Axis (`self.ForwardSpeed`)))
  ;[1 0.1203 0] Forward Handler
  (`Pawn.AddMovementInput` _returnvalue (`KismetMathLibrary.GetForwardVector` (`KismetMathLibrary.MakeRotator` 0.0 0.0 (.yaw (`Pawn.GetControlRotation` _returnvalue)))) _returnvalue_2 false)
  (set `self.PositionOffset` (* _returnvalue_2 (`GameplayStatics.GetWorldDeltaSeconds`))))

(event `Right Handler`
  (params (Axis :type "Float (double-precision)"))
  (bind _returnvalue (`GameplayStatics.GetPlayerPawn` 0))
  (bind _returnvalue_2 (* Axis (`self.TurnSpeed`)))
  ;[1 0.07657 0] Turning Handler
  (`Pawn.AddMovementInput` _returnvalue (`KismetMathLibrary.GetRightVector` (`KismetMathLibrary.MakeRotator` 0.0 0.0 (.yaw (`Pawn.GetControlRotation` _returnvalue)))) _returnvalue_2 false)
  (set `self.TurnOffset` (* _returnvalue_2 (`self.Turn Fudge Factor`))))

(event `UpdateTreadUVs`
  ;[0 0 0] Offset L
  (bind _output_get (set `self.OffsetL` (+ (`self.OffsetL`) (+ (* (`self.TreadDirectionL`) (`self.TurnOffset`)) (`self.PositionOffset`)))))
  (set `self.UVOffsetL` (/ _output_get (/ (`self.TreadLength`) (`self.TreadUVTiles`))))
  ;[0 0 0] OffsetR
  (bind _output_get_2 (set `self.OffsetR` (+ (`self.OffsetR`) (+ (* (`self.TreadDirectionR`) (`self.TurnOffset`)) (`self.PositionOffset`)))))
  (set `self.UVOffsetR` (/ _output_get_2 (/ (`self.TreadLength`) (`self.TreadUVTiles`)))))