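; Tank component that computes a turret aiming yaw for BP_Player from its world cursor.
; TurretAiming stores the look-at yaw from CursorToWorld to the mesh's Turret_Joint socket in ZOffset and prints it, alongside a zero-length debug trace.
; A second sequence branch places the cursor at the mouse hit, oriented to the surface normal.
; The event graph is empty, and nothing here rotates the turret.
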(event `self.ReceiveTick`
  (params (DeltaSeconds :type "Float (single-precision)")))

(fn `TurretAiming`
  (bind (_bblockinghit _binitialoverlap _time _distance _location _impactpoint _normal _impactnormal) (`GameplayStatics.BreakHitResult` (`PlayerController.GetHitResultUnderCursorByChannel` (`GameplayStatics.GetPlayerController` 0) "TraceTypeQuery1" true)))
  (bind _asbp_player (cast `/Game/BLUEPRINTS/PLAYER/BP_Player` (`GameplayStatics.GetPlayerPawn` 0)))
  (bind _output_get (set `self.Player` _asbp_player))
  (set `self.Character` _output_get)
  (`|ExecutionSequence`
    (:`then_0`
      (bind _cursortoworld (`/Game/BLUEPRINTS/PLAYER/BP_Player.CursorToWorld` _output_get))
      (bind _returnvalue (`SceneComponent.K2_GetComponentLocation` _cursortoworld))
      (`KismetSystemLibrary.LineTraceSingle` :`Start` _returnvalue :`End` _returnvalue :`TraceChannel` "TraceTypeQuery1" :`DrawDebugType` "ForOneFrame")
      (bind (_returnvalue_roll _returnvalue_pitch _returnvalue_yaw) (`KismetMathLibrary.BreakRotator` (`KismetMathLibrary.FindLookAtRotation` _returnvalue (`SceneComponent.GetSocketLocation` (`Character.Mesh` (`self.Player`)) "Turret_Joint"))))
      (bind _output_get_2 (set `self.ZOffset` _returnvalue_yaw))
      (`KismetSystemLibrary.PrintString` (`KismetStringLibrary.Conv_DoubleToString` _output_get_2))
      (return))
    (:`then_1`
      (`SceneComponent.K2_SetWorldLocationAndRotation` _cursortoworld _location (`KismetMathLibrary.MakeRotationFromAxes` _impactnormal) false false))))