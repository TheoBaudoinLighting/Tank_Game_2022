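; TraceEquation is an actor Blueprint that visualizes a line trace bouncing off the surface in front of it.
; Every tick it traces forward on the Visibility channel and, if the hit is closer than CheckDistRange, mirrors the trace direction about the hit normal.
; A second trace runs along that reflection, ignoring the hit actor.
; Both traces draw debug lines, and the reflected trace's result is unused.
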(event `self.ReceiveTick`
  (params (DeltaSeconds :type "Float (single-precision)"))
  (bind _returnvalue (`self.K2_GetActorLocation`))
  (bind (_outhit _returnvalue_2) (`KismetSystemLibrary.LineTraceSingle` :`Start` _returnvalue :`End` (+ _returnvalue (* (`self.GetActorForwardVector`) 2000.0)) :`TraceChannel` "TraceTypeQuery1" :`DrawDebugType` "ForDuration"))
  (if _returnvalue_2
    (bind (_bblockinghit _binitialoverlap _time _distance _location _impactpoint _normal _impactnormal _physmat _hitactor _hitcomponent _hitbonename _hititem _elementindex _faceindex _tracestart _traceend) (`GameplayStatics.BreakHitResult` _outhit))
    (if (< _distance (`self.CheckDistRange`))
      (`KismetSystemLibrary.LineTraceSingle` _location (+ _location (* (`KismetMathLibrary.GetReflectionVector` (`KismetMathLibrary.GetDirectionUnitVector` _tracestart _traceend) _normal) 2000.0)) "TraceTypeQuery1" false (`|MakeArray` _hitactor) "ForOneFrame"))))

(fn `UserConstructionScript`)