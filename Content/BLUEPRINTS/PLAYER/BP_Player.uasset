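; BP_Player is the player tank, with cursor-driven turret aim, shooting, health and a random reachable target point for missiles.
; Input axes feed BPMotor00, whose tread UV offsets drive a material parameter collection for track scrolling.
; Tick places the cursor marker on the surface under the mouse and derives turret yaw from it.
; Left click plays the shoot montage and fires through ACShootSystem; damage lowers health, with death handling unwired.
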(event `self.ReceiveBeginPlay`
  ;[0.2578 1 0] Setup Player
  (`parent.ReceiveBeginPlay`)
  (`KismetSystemLibrary.K2_SetTimer` null "TargetProjectilePlayer" 3.0 true)
  (`self.MakeNoise` 1.0 null (0.0 0.0 0.0) 5000.0))

(event `self.ReceiveTick`
  (params (DeltaSeconds :type "Float (single-precision)"))
  (bind _returnvalue (`SceneComponent.K2_GetComponentLocation` (`self.CursorToWorld`)))
  (bind (_returnvalue_roll _returnvalue_pitch _returnvalue_yaw) (`KismetMathLibrary.BreakRotator` (`KismetMathLibrary.FindLookAtRotation` _returnvalue (`SceneComponent.GetSocketLocation` (`self.Mesh`) "Turret_Joint"))))
  (bind (_bblockinghit _binitialoverlap _time _distance _location _impactpoint _normal _impactnormal) (`GameplayStatics.BreakHitResult` (`PlayerController.GetHitResultUnderCursorByChannel` (`GameplayStatics.GetPlayerController` 0) "TraceTypeQuery1" true)))
  ;[0 1 0.9388] Target Logic Player Only
  (`SceneComponent.K2_SetWorldLocationAndRotation` (`self.CursorToWorld`) _location (`KismetMathLibrary.MakeRotationFromAxes` _impactnormal) false false)
  (`KismetSystemLibrary.LineTraceSingle` _returnvalue _returnvalue "TraceTypeQuery1" false (`self.Actors to Ignore`) (`self.Draw Debug Type`))
  (set `self.ZOffset` _returnvalue_yaw))

(event `InputAxis|MoveForward`
  (params (AxisValue :type "Float (single-precision)"))
  (bind _bp_motor_00 (`self.BP_Motor_00`))
  ;[1 0 0] Setup Input
  (`/Game/BLUEPRINTS/BASE_BP/AC_Tank/AC_Motor_00.Forward Handler` (`self.BP_Motor_00`) AxisValue)
  ;[1 1 1] Test Track Logic 01
  (`/Game/BLUEPRINTS/BASE_BP/AC_Tank/AC_Motor_00.UpdateTreadUVs` _bp_motor_00)
  (`KismetMaterialLibrary.SetScalarParameterValue` "/Game/MAT/TANK_M/MPC_TrackTank.MPC_TrackTank" "VOffsetL" (* (`/Game/BLUEPRINTS/BASE_BP/AC_Tank/AC_Motor_00.UVOffsetL` _bp_motor_00) 10.0))
  (`KismetMaterialLibrary.SetScalarParameterValue` "/Game/MAT/TANK_M/MPC_TrackTank.MPC_TrackTank" "VOffsetR" (* (`/Game/BLUEPRINTS/BASE_BP/AC_Tank/AC_Motor_00.UVOffsetR` (`self.BP_Motor_00`)) 10.0)))

(event `InputAxis|MoveRight`
  (params (AxisValue :type "Float (single-precision)"))
  ;[1 0 0] Setup Input
  (`/Game/BLUEPRINTS/BASE_BP/AC_Tank/AC_Motor_00.Right Handler` (`self.BP_Motor_00`) AxisValue))

(event `Shoot`
  (params (Owner :type "Pawn Object Reference"))
  (bind _bulletdirection (`self.BulletDirection`))
  ;[0.9636 1 0] Shoot Logic
  (`self.PlayAnimMontage` "/Game/ANIMATION/TANK/Tank_Shoot_Montage.Tank_Shoot_Montage")
  (`/Game/BLUEPRINTS/BASE_BP/AC_Tank/AC_ShootSystem.Shoot` (`self.AC_ShootSystem`) (`KismetMathLibrary.MakeTransform` (`SceneComponent.K2_GetComponentLocation` _bulletdirection) (`KismetMathLibrary.MakeRotFromZ` (`SceneComponent.GetForwardVector` _bulletdirection))) Owner (`self.ShotColorDebug`)))

(event `Key|LeftMouseButton`
  (params (Key :type "Key Structure"))
  ;[1 1 1] Debug
  (:`Pressed`
    (`self.Shoot` (`GameplayStatics.GetPlayerPawn` 0))))

(event `self.ReceiveAnyDamage`
  (params (Damage :type "Float (single-precision)") (DamageType :type "DamageType Object Reference") (InstigatedBy :type "Controller Object Reference") (DamageCauser :type "Actor Object Reference"))
  ;[1 0 0] Set up Health and damage
  (bind _output_get (set `self.Health` (- (`self.Health`) Damage)))
  (if (== _output_get 0.0)
    _))

(event `Key|Escape`
  (params (Key :type "Key Structure"))
  ;[1 1 1] Quit game
  (:`Pressed`
    (`KismetSystemLibrary.QuitGame` null "Quit")))

(fn `IsAlive?`
  (returns (`Alive?` :type Boolean))
  (return (> (`self.Health`) 0.0)))

(fn `RandomLocationAroundPlayer`
  (bind _asbp_player (cast `/Game/BLUEPRINTS/PLAYER/BP_Player` (`GameplayStatics.GetPlayerCharacter` 0)))
  (set `self.TargetMissilesLocation` (`NavigationSystemV1.K2_GetRandomReachablePointInRadius` (`self.K2_GetActorLocation` _asbp_player) (`self.TargetRadius`) null null)))

(fn `Server_UpdateAim`
  (params (AimPitch :type "Float (double-precision)") (AimLocation :type "Vector Structure")))

(fn `UserConstructionScript`
  (`parent.UserConstructionScript`))